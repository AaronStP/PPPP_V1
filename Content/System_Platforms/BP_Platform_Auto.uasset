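; Auto-moving platform Blueprint that shuttles back and forth while its Activator is on.
; On BeginPlay it starts a forward move if the Activator is on.
; Each time a move finishes, it waits AutoPlatformDelay, rechecks the Activator and moves in the opposite direction.
; The loop stops when that check finds the Activator off, and nothing in this graph restarts it.
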(event `self.ReceiveBeginPlay`
  (`parent.ReceiveBeginPlay`)
  (if (`/Game/System_Platforms/BP_PlatformActivator.IsOn` (`self.Activator`))
    (`self.PlatformMove` true)))

(event `self.PlatformMoveFinished`
  (params (`Is Forward` :type Boolean))
  (`KismetSystemLibrary.Delay` (`self.AutoPlatformDelay`))
  (if (`/Game/System_Platforms/BP_PlatformActivator.IsOn` (`self.Activator`))
    (`self.PlatformMove` (not `Is Forward`))))

(fn `UserConstructionScript`
  (`parent.UserConstructionScript`))