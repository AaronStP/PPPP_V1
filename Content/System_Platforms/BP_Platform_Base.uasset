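; Base Blueprint for moving platforms that travel between their starting position and the location of a referenced target.
; BeginPlay caches the platform's start position and, if the target is valid, its end position.
; PlatformMove plays or reverses the MovePlatform timeline, which lerps the platform between both points without sweeping.
; On completion it calls PlatformMoveFinished with the travel direction, an event left empty here.
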(event `self.ReceiveBeginPlay`
  (bind _targetlocation (`self.TargetLocation`))
  (set `self.StartLocation` (`SceneComponent.K2_GetComponentLocation` (`self.Platform`)))
  (`/Engine/EditorBlueprintResources/StandardMacros.IsValid` _targetlocation
    (:`Is Valid`
      (set `self.EndLocation` (`SceneComponent.K2_GetComponentLocation` (`/Game/System_Platforms/BP_TargetLocation.DefaultSceneRoot` _targetlocation))))))

(event `PlatformMove`
  (params (IsForward :type Boolean))
  (if IsForward
    (bind (_direction _speed) (`Timeline|MovePlatform` :!label _label)
      (:`Update`
        (`SceneComponent.K2_SetWorldLocation` (`self.Platform`) (`KismetMathLibrary.VLerp` (`self.StartLocation`) (`self.EndLocation`) _speed) false false))
      (:`Finished`
        (`self.PlatformMoveFinished` (select `ETimelineDirection` _direction :`Forward` true))))
    (else
      (goto _label :!via `Reverse`))))

(event `PlatformMoveFinished`
  (params (`Is Forward` :type Boolean)))

(fn `UserConstructionScript`)