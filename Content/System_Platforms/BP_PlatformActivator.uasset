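; BP_PlatformActivator is an interactable lever that switches linked platforms between forward and backward movement.
; Interact plays or reverses the MoveLever timeline based on IsOn, rotating the lever between its initial rotation and a fixed tilt.
; When the timeline finishes, it calls PlatformMove on each valid entry in PlatformsToMove with a boolean derived from timeline direction, then toggles IsOn.
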(event `self.ReceiveBeginPlay`
  (set `self.StartPosition` (`SceneComponent.RelativeRotation` (`self.Lever`))))

(event `/Game/Player/BPI_Interact.Interact`
  (if (`self.IsOn`)
    (bind (_direction _speed) (`Timeline|MoveLever` :!via `Reverse` :!label _label)
      (:`Update`
        (`SceneComponent.K2_SetRelativeRotation` (`self.Lever`) (`KismetMathLibrary.RLerp` (`self.StartPosition`) (struct :`Pitch` 25.0) _speed) false false))
      (:`Finished`
        (`self.ActivateLeverFinished` _direction)
        (if (`self.IsOn`)
          (set `self.IsOn` false)
          (else
            (set `self.IsOn` true)))))
    (else
      (goto _label))))

(fn `ActivateLeverFinished`
  (params (Index :type "ETimelineDirection Enum" :default "Forward"))
  (for _array_element (`self.PlatformsToMove`)
    (`/Engine/EditorBlueprintResources/StandardMacros.IsValid` _array_element
      (:`Is Valid`
        (`/Game/System_Platforms/BP_Platform_Base.PlatformMove` _array_element (select `ETimelineDirection` Index :`Forward` true))))))

(fn `UserConstructionScript`)