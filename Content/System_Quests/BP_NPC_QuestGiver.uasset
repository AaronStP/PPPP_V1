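; BP_NPC_QuestGiver is an NPC actor that gives quests to the player.
; Its TextRender starts hidden and shows only while a BP_Player overlaps the InteractionRadius, acting as a proximity prompt.
; The Interact event passes the player to the BPACQuestGiver component's InteractQuest, which handles the quest interaction.
; The actor's own InteractQuest function is a stub that returns an empty string.
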(event `self.ReceiveBeginPlay`
  (`SceneComponent.SetVisibility` (`self.TextRender`) false false))

(event `self.InteractionRadius.OnComponentBeginOverlap`
  (params (OverlappedComponent :type "PrimitiveComponent Object Reference") (OtherActor :type "Actor Object Reference") (OtherComp :type "PrimitiveComponent Object Reference") (OtherBodyIndex :type Integer) (bFromSweep :type Boolean) (SweepResult :type "HitResult Structure (by ref)"))
  (cast `/Game/Player/Blueprints/BP_Player` OtherActor)
  (`SceneComponent.SetVisibility` (`self.TextRender`) true false))

(event `self.InteractionRadius.OnComponentEndOverlap`
  (params (OverlappedComponent :type "PrimitiveComponent Object Reference") (OtherActor :type "Actor Object Reference") (OtherComp :type "PrimitiveComponent Object Reference") (OtherBodyIndex :type Integer))
  (cast `/Game/Player/Blueprints/BP_Player` OtherActor)
  (`SceneComponent.SetVisibility` (`self.TextRender`) false false))

(event `/Game/Player/BPI_Interact.Interact`
  (params (Player :type "/Game/Player/Blueprints/BP_Player Object Reference"))
  (`/Game/System_Quests/BPAC_QuestGiver.Interact_Quest` (`self.BPAC_QuestGiver`) Player))

(fn `Interact_Quest`
  (params (Player :type "/Game/Player/Blueprints/BP_Player Object Reference"))
  (returns (ObjectiveID :type String))
  (return ""))

(fn `UserConstructionScript`)