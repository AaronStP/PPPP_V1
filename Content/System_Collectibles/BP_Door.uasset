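; BP_Door is an interactable door that can be locked behind a required key and swings open when used.
; On interaction, an unlocked door opens directly, while a locked one opens only if the BP_Player's KeyRing contains the RequiredKey.
; Opening plays a timeline that lerps the door mesh from its BeginPlay relative rotation to a fixed target rotation, with no closing logic.
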(event `self.ReceiveBeginPlay`
  ;[1 1 1] Set StartPos
  (set `self.StartingPosition` (`SceneComponent.RelativeRotation` (`self.DoorMesh`))))

(event `/Game/Player/BPI_Interact.Interact`
  (if (`self.IsLocked`)
    (bind _returnvalue (`GameplayStatics.GetActorOfClass` "/Game/Player/Blueprints/BP_Player.BP_Player_C"))
    (if (`KismetArrayLibrary.Array_Contains` (`/Game/Player/Blueprints/BP_Player.KeyRing` _returnvalue) (`self.RequiredKey`))
      (`self.OpenDoor`))
    (else
      (`self.OpenDoor`))))

(event `OpenDoor`
  (bind (_direction _speed) (`Timeline|TL_OpenDoor`)
    (:`Update`
      (`SceneComponent.K2_SetRelativeRotation` (`self.DoorMesh`) (`KismetMathLibrary.RLerp` (`self.StartingPosition`) (struct :`Yaw` -90.0) _speed) false false))))

(fn `UserConstructionScript`)